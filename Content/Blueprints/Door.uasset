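; Numbered sliding door actor that opens once when an Activate event carries its matching door number.
; BeginPlay caches the closed and open positions and keeps Tick disabled until Open enables it, with CanChange blocking repeat calls.
; Tick slides the mesh along local X by Speed until it nears the open location, then sets IsOpen and disables itself.
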(event `self.ReceiveTick`
  (params (DeltaSeconds :type "Float (single-precision)"))
  (if (`self.Is Open`)
    (bind _result (`/Engine/EditorBlueprintResources/StandardMacros.NegateFloat` (`self.Open Distance`))
      (:`  `
        (`SceneComponent.K2_AddLocalOffset` (`self.Door mesh`) (`KismetMathLibrary.MakeVector` _result) false false)
        (set `self.Is Open` false)
        (`self.SetActorTickEnabled` false :!label _label)))
    (elif (!= (`SceneComponent.RelativeLocation` (`self.Door mesh`)) (`self.Open Location`) :`ErrorTolerance` 0.5)
      (`SceneComponent.K2_AddLocalOffset` (`self.Door mesh`) (`KismetMathLibrary.MakeVector` (* DeltaSeconds (`self.Speed`))) false false)
      (else
        (set `self.Is Open` true)
        (goto _label)))))

(event `self.ReceiveBeginPlay`
  (`self.SetActorTickEnabled` false)
  (bind _output_get (set `self.Closed Location` (`SceneComponent.RelativeLocation` (`self.Door mesh`))))
  (set `self.Open Location` (+ _output_get (`KismetMathLibrary.MakeVector` (`self.Open Distance`)))))

(event `/Game/Blueprints/DoorInteractionInterface.Activate`
  (params (Activated :type Boolean) (InNo :type Integer) (TimesActivated :type Integer))
  (if (and Activated (== InNo (`self.Door No`)))
    (`self.Open`)))

(fn `Open`
  (if (`self.Can Change`)
    (`self.SetActorTickEnabled` true)
    (set `self.Can Change` false)))

(fn `UserConstructionScript`)