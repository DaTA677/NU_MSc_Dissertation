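; Trigger actor that starts a countdown when the first-person character first overlaps it, and can open a linked door when time runs out.
; It reuses or creates the timer widget held by PuzzleGameInstance, shows it if ShowTimer is set, and polls it on Tick.
; Tick displays optional HUD story text at a set elapsed time.
; On expiry (door opens only with ShowTimer) or when the door becomes unchangeable, it self-destructs.
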(event `self.ReceiveTick`
  (params (DeltaSeconds :type "Float (single-precision)"))
  (bind _timerref (`self.TimerRef`))
  (bind _door (`self.Door`))
  (bind _returnvalue (>= (`/Game/FirstPerson/Blueprints/Timer.Time_Val` _timerref) 0))
  (`/Engine/EditorBlueprintResources/StandardMacros.IsValid` _door
    (:`Is Valid`
      (if (`/Game/Blueprints/Door.Can Change` _door)
        (if _returnvalue
          (if (and (not (`KismetTextLibrary.TextIsEmpty` (`self.StoryText`))) (== (`self.TimeToDisplayStory`) (- (`self.TimerSeconds`) (`/Game/FirstPerson/Blueprints/Timer.Time_Val` (`self.TimerRef`))))) :!label _label
            (bind _aspuzzle_game_instance (cast `/Game/Blueprints/PuzzleGameInstance` (`GameplayStatics.GetGameInstance`)))
            (bind _hud (`/Game/Blueprints/PuzzleGameInstance.HUD` _aspuzzle_game_instance))
            (set `MultiLineEditableTextBox.Text` (`self.StoryText`) (`TrialGameUI.StoryText` _hud))
            (set `TrialGameUI.StoryTextDelayTime` 10.0 _hud)
            (set `TrialGameUI.bShowStoryText` true _hud)
            (`/Game/FirstPerson/Blueprints/BP_GameUI.ShowStory` _hud))
          (else
            (`/Game/FirstPerson/Blueprints/Timer.StopTimer` _timerref :!label _label_2)
            (`self.SetActorTickEnabled` false)
            (`self.OpenDoor`)
            (`self.SetLifeSpan` 0.2 :!label _label_3)
            (bind _aspuzzle_game_instance_2 (cast `/Game/Blueprints/PuzzleGameInstance` (`GameplayStatics.GetGameInstance`)))
            (`/Game/Blueprints/PuzzleGameInstance.ChangeStoryState` _aspuzzle_game_instance_2 false)))
        (else
          (`/Game/FirstPerson/Blueprints/Timer.StopTimer` _timerref)
          (`self.SetActorTickEnabled` false)
          (goto _label_3))))
    (:`Is Not Valid`
      (if _returnvalue
        (goto _label)
        (else
          (goto _label_2))))))

(event `self. TriggerChange.OnComponentBeginOverlap`
  (params (OverlappedComponent :type "PrimitiveComponent Object Reference") (OtherActor :type "Actor Object Reference") (OtherComp :type "PrimitiveComponent Object Reference") (OtherBodyIndex :type Integer) (bFromSweep :type Boolean) (SweepResult :type "HitResult Structure (by ref)"))
  (cast `/Game/FirstPerson/Blueprints/BP_FirstPersonCharacter` OtherActor)
  (if (not (`self.IsOverlapped`))
    (set `self.IsOverlapped` true)
    (bind _aspuzzle_game_instance (cast `/Game/Blueprints/PuzzleGameInstance` (`GameplayStatics.GetGameInstance`)))
    (`/Engine/EditorBlueprintResources/StandardMacros.IsValid` (`/Game/Blueprints/PuzzleGameInstance.TimerUI` _aspuzzle_game_instance)
      (:`Is Valid`
        (bind _timerui (`/Game/Blueprints/PuzzleGameInstance.TimerUI` _aspuzzle_game_instance))
        (set `/Game/FirstPerson/Blueprints/Timer.Time_Val` (`self.TimerSeconds`) _timerui)
        (set `self.TimerRef` _timerui))
      (:`Is Not Valid`
        (bind _returnvalue (`|CreateWidget` "/Game/FirstPerson/Blueprints/Timer.Timer_C"))
        (bind _output_get (set `/Game/Blueprints/PuzzleGameInstance.TimerUI` _returnvalue _aspuzzle_game_instance))
        (set `self.TimerRef` _output_get)
        (set `/Game/FirstPerson/Blueprints/Timer.Time_Val` (`self.TimerSeconds`) _output_get)))
    (`/Game/FirstPerson/Blueprints/Timer.RunTimer` _timerui)
    (`self.SetActorTickEnabled` true)
    (if (`self.ShowTimer`)
      (`UserWidget.AddToViewport` _timerui 0))))

(fn `OpenDoor`
  (bind _door (`self.Door`))
  (if (and (`KismetSystemLibrary.IsValid` (`self.Door`)) (`self.ShowTimer`) (`self.IsOverlapped`) (not (`self.IsActorTickEnabled`)))
    (message `/Game/Blueprints/DoorInteractionInterface.Activate` _door true (`/Game/Blueprints/Door.Door No` _door) 1)))

(fn `UserConstructionScript`)