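; StoryTrigger is a placeable actor that shows story text on the player's HUD when they enter its trigger.
; Overlapping TriggerChange casts to BP_FirstPersonCharacter and its BP_GameUI, passes in DisplayText and DisplayDuration, then calls ShowStory.
; It then sets a short lifespan so the trigger removes itself after use.
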(event `self. TriggerChange.OnComponentBeginOverlap`
  (params (OverlappedComponent :type "PrimitiveComponent Object Reference") (OtherActor :type "Actor Object Reference") (OtherComp :type "PrimitiveComponent Object Reference") (OtherBodyIndex :type Integer) (bFromSweep :type Boolean) (SweepResult :type "HitResult Structure (by ref)"))
  (bind _asbp_first_person_character (cast `/Game/FirstPerson/Blueprints/BP_FirstPersonCharacter` OtherActor))
  (bind _asbp_game_ui (cast `/Game/FirstPerson/Blueprints/BP_GameUI` (`PuzzleGameCharacter.HUD` _asbp_first_person_character)))
  (set `MultiLineEditableTextBox.Text` (`self.DisplayText`) (`TrialGameUI.StoryText` _asbp_game_ui))
  (set `TrialGameUI.bShowStoryText` true _asbp_game_ui)
  (set `TrialGameUI.StoryTextDelayTime` (`self.DisplayDuration`) _asbp_game_ui)
  (`/Game/FirstPerson/Blueprints/BP_GameUI.ShowStory` _asbp_game_ui)
  (`self.SetLifeSpan` 2.0))

(fn `UserConstructionScript`)