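; Information trigger volume that shows an instructional popup when the first-person player character walks into it.
; On overlap it reuses the Information widget cached on PuzzleGameInstance, or creates and caches one, then fills it with its heading and instruction text.
; It hides the HUD, shows the mouse cursor and pauses the game.
; A short life span makes each trigger one-shot.
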(event `self. TriggerChange.OnComponentBeginOverlap`
  (params (OverlappedComponent :type "PrimitiveComponent Object Reference") (OtherActor :type "Actor Object Reference") (OtherComp :type "PrimitiveComponent Object Reference") (OtherBodyIndex :type Integer) (bFromSweep :type Boolean) (SweepResult :type "HitResult Structure (by ref)"))
  (cast `/Game/FirstPerson/Blueprints/BP_FirstPersonCharacter` OtherActor)
  (bind _aspuzzle_game_instance (cast `/Game/Blueprints/PuzzleGameInstance` (`GameplayStatics.GetGameInstance`)))
  (`/Engine/EditorBlueprintResources/StandardMacros.IsValid` (`/Game/Blueprints/PuzzleGameInstance.InformationUIRef` _aspuzzle_game_instance)
    (:`Is Valid`
      (bind _informationuiref (`/Game/Blueprints/PuzzleGameInstance.InformationUIRef` _aspuzzle_game_instance))
      (`/Game/FirstPerson/Blueprints/Information.SetInformationText` _informationuiref (`self.InstructionText`))
      (`/Game/FirstPerson/Blueprints/Information.SetInformationTitle` _informationuiref (`self.HeadingText`))
      (`UserWidget.AddToViewport` _informationuiref 0))
    (:`Is Not Valid`
      (bind _returnvalue (`|CreateWidget` "/Game/FirstPerson/Blueprints/Information.Information_C"))
      (bind _output_get (set `/Game/Blueprints/PuzzleGameInstance.InformationUIRef` _returnvalue _aspuzzle_game_instance))
      (`/Game/FirstPerson/Blueprints/Information.SetInformationText` _output_get (`self.InstructionText`))
      (`/Game/FirstPerson/Blueprints/Information.SetInformationTitle` _output_get (`self.HeadingText`))
      (`UserWidget.AddToViewport` _output_get 0)))
  (`Widget.SetVisibility` (`/Game/Blueprints/PuzzleGameInstance.HUD` _aspuzzle_game_instance) "Hidden")
  (set `PlayerController.bShowMouseCursor` true (`GameplayStatics.GetPlayerController` 0))
  (`GameplayStatics.SetGamePaused` true)
  (`self.SetLifeSpan` 0.2))

(fn `UserConstructionScript`)