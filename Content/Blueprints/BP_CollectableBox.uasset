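; BP_CollectableBox is a collectable box actor that a character picks up through its InteractComponent.
; On interact, it casts the interacted actor to BP_CollectableBox, calls Collect with the picking character, then hides that box after a short delay.
; Collect is not defined in these graphs, and a distance check against the interact sphere radius is left unconnected.
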(event `self.InteractComponent.OnInteract`
  (params (PickUpCharacter :type "PuzzleGameCharacter Object Reference") (CurrentActor :type "Actor Object Reference"))
  (bind _asbp_collectable_box (cast `/Game/Blueprints/BP_CollectableBox` CurrentActor))
  (`self.Collect` _asbp_collectable_box PickUpCharacter)
  (`KismetSystemLibrary.Delay` 0.2)
  (`self.SetActorHiddenInGame` _asbp_collectable_box true))

(fn `UserConstructionScript`)