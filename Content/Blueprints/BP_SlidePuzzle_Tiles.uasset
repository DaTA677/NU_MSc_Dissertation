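; Tile actor for a sliding puzzle, meant to show one cell of a 4x4 texture grid.
; On construction it takes its number from a shared counter in SlidePuzzleState and increments it, logging if the cast fails.
; Construction, BeginPlay and every Tick read the static mesh's UVs and offset them by the tile's quarter-step cell.
; The edited UVs are never written back to a mesh.
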(event `self.ReceiveBeginPlay`
  (bind _returnvalue (mod (`self.TileNo`) 16))
  (bind (_vertices _triangles _normals _uvs) (`KismetProceduralMeshLibrary.GetSectionFromStaticMesh` (`StaticMeshComponent.StaticMesh` (`self.StaticMeshComponent`)) :!label _label))
  (for _array_element _uvs
    (bind (_x _y) (`KismetMathLibrary.BreakVector2D` (+ _array_element (`KismetMathLibrary.MakeVector2D` (* (`KismetMathLibrary.Conv_IntToDouble` (mod _returnvalue 4)) 0.25) (* (`KismetMathLibrary.Conv_IntToDouble` (/ _returnvalue 4)) 0.25)))))
    (`KismetMathLibrary.Set2D` _array_element _x _y)))

(event `self.ReceiveTick`
  (params (DeltaSeconds :type "Float (single-precision)"))
  (goto _label))

(fn `UserConstructionScript`
  (bind _asslide_puzzle_state (cast `/Game/Blueprints/SlidePuzzleState` (`GameplayStatics.GetGameState`))
    (:`then`
      (bind _tilescreated (`/Game/Blueprints/SlidePuzzleState.TilesCreated` _asslide_puzzle_state))
      (bind _output_get (set `self.TileNo` _tilescreated))
      (set `/Game/Blueprints/SlidePuzzleState.TilesCreated` (+ _tilescreated 1) _asslide_puzzle_state)
      (bind (_vertices _triangles _normals _uvs) (`KismetProceduralMeshLibrary.GetSectionFromStaticMesh` (`StaticMeshComponent.StaticMesh` (`self.StaticMeshComponent`))))
      (for _array_element _uvs
        (bind _returnvalue (mod _output_get 16))
        (bind (_x _y) (`KismetMathLibrary.BreakVector2D` (+ _array_element (`KismetMathLibrary.MakeVector2D` (* (`KismetMathLibrary.Conv_IntToDouble` (mod _returnvalue 4)) 0.25) (* (`KismetMathLibrary.Conv_IntToDouble` (/ _returnvalue 4)) 0.25)))))
        (`KismetMathLibrary.Set2D` _array_element _x _y)))
    (:`CastFailed`
      (`KismetSystemLibrary.LogString` "Cant Update slide values"))))