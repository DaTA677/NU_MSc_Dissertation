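; A clickable number pad pawn that shows the mouse cursor when possessed and checks an entered code against a stored one.
; Digit clicks fill an array, with 1-9 derived from the key's position relative to the mesh and 0 added directly.
; The length check allows a fifth digit, while Back removes the last.
; Enter requires four digits, sums each times ten rather than by place value, logs the result and clears wrong entries.
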(event `self.ReceivePossessed`
  (params (NewController :type "Controller Object Reference"))
  (bind _asplayer_controller (cast `PlayerController` NewController))
  (set `PlayerController.bShowMouseCursor` true _asplayer_controller))

(event `self.1.OnClicked`
  (params (TouchedComponent :type "PrimitiveComponent Object Reference") (ButtonPressed :type "Key Structure"))
  (`self.AddValueToEnteredStringArray` TouchedComponent))

(event `self.2.OnClicked`
  (params (TouchedComponent :type "PrimitiveComponent Object Reference") (ButtonPressed :type "Key Structure"))
  (`self.AddValueToEnteredStringArray` TouchedComponent))

(event `self.3.OnClicked`
  (params (TouchedComponent :type "PrimitiveComponent Object Reference") (ButtonPressed :type "Key Structure"))
  (`self.AddValueToEnteredStringArray` TouchedComponent))

(event `self.4.OnClicked`
  (params (TouchedComponent :type "PrimitiveComponent Object Reference") (ButtonPressed :type "Key Structure"))
  (`self.AddValueToEnteredStringArray` TouchedComponent))

(event `self.5.OnClicked`
  (params (TouchedComponent :type "PrimitiveComponent Object Reference") (ButtonPressed :type "Key Structure"))
  (`self.AddValueToEnteredStringArray` TouchedComponent))

(event `self.6.OnClicked`
  (params (TouchedComponent :type "PrimitiveComponent Object Reference") (ButtonPressed :type "Key Structure"))
  (`self.AddValueToEnteredStringArray` TouchedComponent))

(event `self.7.OnClicked`
  (params (TouchedComponent :type "PrimitiveComponent Object Reference") (ButtonPressed :type "Key Structure"))
  (`self.AddValueToEnteredStringArray` TouchedComponent))

(event `self.8.OnClicked`
  (params (TouchedComponent :type "PrimitiveComponent Object Reference") (ButtonPressed :type "Key Structure"))
  (`self.AddValueToEnteredStringArray` TouchedComponent))

(event `self.9.OnClicked`
  (params (TouchedComponent :type "PrimitiveComponent Object Reference") (ButtonPressed :type "Key Structure"))
  (`self.AddValueToEnteredStringArray` TouchedComponent))

(event `self.0.OnClicked`
  (params (TouchedComponent :type "PrimitiveComponent Object Reference") (ButtonPressed :type "Key Structure"))
  (bind (_enteredstring _returnvalue) (`self.CheckEnteredStringArraySize`))
  (if _returnvalue
    (`KismetArrayLibrary.Array_Add` _enteredstring)))

(event `self.Back.OnClicked`
  (params (TouchedComponent :type "PrimitiveComponent Object Reference") (ButtonPressed :type "Key Structure"))
  (bind _enteredstring (`self.EnteredString`))
  (bind _returnvalue (`KismetArrayLibrary.Array_Length` _enteredstring))
  (if (> _returnvalue 0)
    (`KismetArrayLibrary.Array_Remove` _enteredstring (- _returnvalue 1))))

(event `self.Enter.OnClicked`
  (params (TouchedComponent :type "PrimitiveComponent Object Reference") (ButtonPressed :type "Key Structure"))
  (bind _enteredstring (`self.EnteredString`))
  (bind _enterednumber (`self.EnteredNumber`))
  (bind _returnvalue (`KismetArrayLibrary.Array_Length` _enteredstring))
  (if (== _returnvalue 4)
    (set `self.EnteredNumber` 0)
    (for _index (range _returnvalue)
      (set `self.EnteredNumber` (+ _enterednumber (* (`|GetArrayItem` _enteredstring _index) 10))))
    (if (== _enterednumber (`self.FinalCodeString`))
      (`KismetSystemLibrary.LogString` "Correct Code")
      (else
        (`KismetSystemLibrary.LogString` "Incorrect code")
        (`KismetArrayLibrary.Array_Clear` _enteredstring)
        (set `self.EnteredNumber` 0)))))

(fn `AddValueToEnteredStringArray`
  (params (PressedComponent :type "SceneComponent Object Reference"))
  (bind (_enteredstring _returnvalue) (`self.CheckEnteredStringArraySize`))
  (if _returnvalue
    (bind _output_get (`self.GetContactLocation` PressedComponent))
    (`KismetArrayLibrary.Array_Add` _enteredstring (`KismetMathLibrary.Conv_Int64ToInt` _output_get))))

(fn `CheckEnteredStringArraySize`
  (returns (EnteredString :type "Array of Integer") (ReturnValue :type Boolean))
  (bind _enteredstring (`self.EnteredString`))
  (return _enteredstring (<= (`KismetArrayLibrary.Array_Length` _enteredstring) 4)))

(fn `GetContactLocation`
  (params (PressedComponent :type "SceneComponent Object Reference"))
  (returns (Output_Get :type Integer64))
  (bind _y (.y (- (`SceneComponent.K2_GetComponentLocation` PressedComponent) (`SceneComponent.K2_GetComponentLocation` (`self.RenderedMesh`)))))
  (if (== _y -60.0)
    (set `self.Y` 0)
    (elif (== _y 0.0)
      (set `self.Y` 1)
      (else
        (set `self.Y` 2))))
  (bind _output_get (set `self.ContactLocation` (+ (* (`.ReturnValue` (`KismetMathLibrary.FMod64` (- (.x (- (`SceneComponent.K2_GetComponentLocation` PressedComponent) (`SceneComponent.K2_GetComponentLocation` (`self.RenderedMesh`)))) 60.0) -40.0)) 3) (`self.Y`) 1)))
  (return _output_get))

(fn `UserConstructionScript`)